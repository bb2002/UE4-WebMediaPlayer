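; Player pawn for the example levels that sets up the media controller UI for the web audio and web video demos.
; On BeginPlay it checks the current level name and adds either the audio or the video controller widget to the viewport.
; It then binds the widget to the level's example radio or TV actor, only when exactly one such actor exists.
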(event EventBeginPlay
  (bind _returnvalue (Game|GetPlayerController 0))
  ;[1 1 1] Create Controller Widget
  (bind _returnvalue_2 (Game|GetCurrentLevelName true))
  (switch string _returnvalue_2
    (:WebAudioExample
      (bind _returnvalue_3 (UserInterface|CreateWidget "/WebMediaPlayer/ExampleLevel/Contents/AudioController_Widget.AudioController_Widget_C" _returnvalue))
      (UserInterface|Viewport|AddtoViewport _returnvalue_3 0)
      (bind _outactors (Actor|GetAllActorsOfClass "/WebMediaPlayer/ExampleLevel/Contents/BP_ExampleRadio.BP_ExampleRadio_C"))
      (if (== (Utilities|Array|Length _outactors) 1)
        (Default|SetupAudioPlayer _returnvalue_3 (Utilities|Array|Get(acopy) _outactors))))
    (:WebVideoExample
      (bind _returnvalue_4 (UserInterface|CreateWidget "/WebMediaPlayer/ExampleLevel/Contents/VideoController_Widget.VideoController_Widget_C" _returnvalue))
      (UserInterface|Viewport|AddtoViewport _returnvalue_4 0)
      (bind _outactors_2 (Actor|GetAllActorsOfClass "/WebMediaPlayer/ExampleLevel/Contents/BP_ExampleTV.BP_ExampleTV_C"))
      (if (== (Utilities|Array|Length _outactors_2) 1)
        (Default|SetupVideoPlayer _returnvalue_4 (Utilities|Array|Get(acopy) _outactors_2))))))

(event Collision|EventActorBeginOverlap
  (params (OtherActor :type Actor%20Object%20Reference)))

(event EventTick
  (params (DeltaSeconds :type Float%20%28single-precision%29)))

(fn ConstructionScript)